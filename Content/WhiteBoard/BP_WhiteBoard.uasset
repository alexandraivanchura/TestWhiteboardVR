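; Grabbable whiteboard actor that can be drawn on with colored brushes and wiped clean.
; On BeginPlay it creates a white render target, shows it through a dynamic canvas material and creates a dynamic brush material.
; Draw events pass color, size and normalized location to DrawBrush, which stamps the brush onto the render target via canvas drawing.
; Tick keeps the board upright by zeroing pitch and roll while preserving yaw.
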(event `self.ReceiveBeginPlay`
  (`|ExecutionSequence`
    (:`then_0`
      (bind _returnvalue (`KismetRenderingLibrary.CreateRenderTarget2D` 2048 2048 "RTF_RGBA16f" (struct :`R` 1.0 :`G` 1.0 :`B` 1.0 :`A` 1.0)))
      (bind _output_get (set `self.RenderTarget` _returnvalue))
      (`KismetRenderingLibrary.ClearRenderTarget2D` _output_get (struct :`R` 1.0 :`G` 1.0 :`B` 1.0 :`A` 1.0)))
    (:`then_1`
      (bind _returnvalue_2 (`KismetMaterialLibrary.CreateDynamicMaterialInstance` "/Game/WhiteBoard/M_Canvas.M_Canvas"))
      (`MaterialInstanceDynamic.SetTextureParameterValue` _returnvalue_2 "RenderTarget" (`self.RenderTarget`))
      (`PrimitiveComponent.SetMaterial` (`self.Whiteboard`) 0 _returnvalue_2))
    (:`then_2`
      (bind _returnvalue_3 (`KismetMaterialLibrary.CreateDynamicMaterialInstance` "/Game/WhiteBoard/M_Brush.M_Brush"))
      (set `self.WhiteBoardMarker_MI` _returnvalue_3))))

(event `CleanWhiteboard`
  (`KismetRenderingLibrary.ClearRenderTarget2D` (`self.RenderTarget`) (struct :`R` 1.0 :`G` 1.0 :`B` 1.0 :`A` 1.0)))

(event `DrawOnWhiteBoard`
  (params (DrawingLocation :type "Vector2D Structure") (Color :type "/Game/WhiteBoard/E_MarkerColors Enum" :default "NewEnumerator0") (DrawingSize :type "Float (double-precision)" :default 30.0))
  (`self.DrawBrush` Color DrawingSize DrawingLocation))

(event `self.GrabComponent.OnGrabbed`)

(event `self.ReceiveTick`
  (params (DeltaSeconds :type "Float (single-precision)"))
  (bind _whiteboard (`self.Whiteboard`))
  (bind (_returnvalue_roll _returnvalue_pitch _returnvalue_yaw) (`KismetMathLibrary.BreakRotator` (`SceneComponent.K2_GetComponentRotation` _whiteboard)))
  (`SceneComponent.K2_SetWorldRotation` _whiteboard (`KismetMathLibrary.MakeRotator` 0.0 0.0 _returnvalue_yaw) false false))

(fn `DrawBrush`
  (params (BrushColor :type "/Game/WhiteBoard/E_MarkerColors Enum" :default "NewEnumerator0") (BrushSize :type "Float (double-precision)") (DrawLocation :type "Vector2D Structure"))
  (bind _whiteboardmarker_mi (`self.WhiteBoardMarker_MI`))
  (bind _brushsize (`local.BrushSize`))
  (`|ExecutionSequence`
    (:`then_0`
      (switch `/Game/WhiteBoard/E_MarkerColors` BrushColor
        (:`NewEnumerator2`
          (`MaterialInstanceDynamic.SetVectorParameterValue` _whiteboardmarker_mi "Color" (struct :`R` 1.0 :`G` 1.0 :`B` 1.0 :`A` 1.0)))
        (:`NewEnumerator0`
          (`MaterialInstanceDynamic.SetVectorParameterValue` _whiteboardmarker_mi "Color" (struct :`G` 0.179629 :`B` 1.0 :`A` 1.0)))
        (:`NewEnumerator1`
          (`MaterialInstanceDynamic.SetVectorParameterValue` _whiteboardmarker_mi "Color" (struct :`R` 1.0 :`B` 0.023477 :`A` 1.0)))))
    (:`then_1`
      (bind (_canvas _size _context) (`KismetRenderingLibrary.BeginDrawCanvasToRenderTarget` (`self.RenderTarget`)))
      (`Canvas.K2_DrawMaterial` _canvas (`self.WhiteBoardMarker_MI`) (- (* _size (`local.DrawLocation`)) (/ _brushsize 2.0)) (`KismetMathLibrary.Conv_DoubleToVector2D` _brushsize) (0.0 0.0) (1.0 1.0) 0.0 (0.5 0.5))
      (`KismetRenderingLibrary.EndDrawCanvasToRenderTarget` _context))))

(fn `UserConstructionScript`)