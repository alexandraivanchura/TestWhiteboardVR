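; Whiteboard marker actor with a colored tip (blue or red material set on BeginPlay) and an eraser, for drawing on and wiping BP_WhiteBoard.
; Tip and Eraser overlaps toggle drawing and erasing, with drawing taking priority.
; While active, Tick line-traces along the Start–End axis toward the respective end and converts the hit to a collision UV.
; It passes that UV to DrawOnWhiteBoard, with erasing done as larger white strokes.
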(event `self.ReceiveBeginPlay`
  (bind _tip (`self.Tip`))
  (switch `/Game/WhiteBoard/E_MarkerColors` (`self.Color`)
    (:`NewEnumerator0`
      (`PrimitiveComponent.SetMaterial` _tip 0 "/Game/WhiteBoard/M_Blue.M_Blue"))
    (:`NewEnumerator1`
      (`PrimitiveComponent.SetMaterial` _tip 0 "/Game/WhiteBoard/M_Red.M_Red"))))

(event `self.ReceiveTick`
  (params (DeltaSeconds :type "Float (single-precision)"))
  (bind _returnvalue (`SceneComponent.K2_GetComponentLocation` (`self.Start`)))
  (bind _returnvalue_2 (`SceneComponent.K2_GetComponentLocation` (`self.End`)))
  (if (`self.IsDrawing`)
    (bind (_outhit _returnvalue_3) (`KismetSystemLibrary.LineTraceSingle` _returnvalue (+ _returnvalue (* (`KismetMathLibrary.GetDirectionUnitVector` _returnvalue (`SceneComponent.K2_GetComponentLocation` (`self.End`))) 500.0)) "TraceTypeQuery1" true))
    (if _returnvalue_3
      (bind _asbp_white_board (cast `/Game/WhiteBoard/BP_WhiteBoard` (`.HitActor` (`GameplayStatics.BreakHitResult` _outhit))))
      (`/Game/WhiteBoard/BP_WhiteBoard.DrawOnWhiteBoard` _asbp_white_board (`GameplayStatics.FindCollisionUV` _outhit) (`self.Color`) 30.0))
    (elif (`self.IsErasing`)
      (bind (_outhit_2 _returnvalue_4) (`KismetSystemLibrary.LineTraceSingle` _returnvalue_2 (+ _returnvalue_2 (* (`KismetMathLibrary.GetDirectionUnitVector` _returnvalue_2 (`SceneComponent.K2_GetComponentLocation` (`self.Start`))) 500.0)) "TraceTypeQuery1" true))
      (if _returnvalue_4
        (bind _asbp_white_board_2 (cast `/Game/WhiteBoard/BP_WhiteBoard` (`.HitActor` (`GameplayStatics.BreakHitResult` _outhit_2))))
        (`/Game/WhiteBoard/BP_WhiteBoard.DrawOnWhiteBoard` _asbp_white_board_2 (`GameplayStatics.FindCollisionUV` _outhit_2) "NewEnumerator2" 60.0)))))

(event `self.Tip.OnComponentBeginOverlap`
  (params (OverlappedComponent :type "PrimitiveComponent Object Reference") (OtherActor :type "Actor Object Reference") (OtherComp :type "PrimitiveComponent Object Reference") (OtherBodyIndex :type Integer) (bFromSweep :type Boolean) (SweepResult :type "HitResult Structure (by ref)"))
  (set `self.IsDrawing` true))

(event `self.Tip.OnComponentEndOverlap`
  (params (OverlappedComponent :type "PrimitiveComponent Object Reference") (OtherActor :type "Actor Object Reference") (OtherComp :type "PrimitiveComponent Object Reference") (OtherBodyIndex :type Integer))
  (set `self.IsDrawing` false))

(event `self.Eraser.OnComponentBeginOverlap`
  (params (OverlappedComponent :type "PrimitiveComponent Object Reference") (OtherActor :type "Actor Object Reference") (OtherComp :type "PrimitiveComponent Object Reference") (OtherBodyIndex :type Integer) (bFromSweep :type Boolean) (SweepResult :type "HitResult Structure (by ref)"))
  (set `self.IsErasing` true))

(event `self.Eraser.OnComponentEndOverlap`
  (params (OverlappedComponent :type "PrimitiveComponent Object Reference") (OtherActor :type "Actor Object Reference") (OtherComp :type "PrimitiveComponent Object Reference") (OtherBodyIndex :type Integer))
  (set `self.IsErasing` false))

(fn `UserConstructionScript`)